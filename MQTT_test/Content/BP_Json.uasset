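; BP_Json is an actor Blueprint that polls a JSON file and turns its "happy1" entry into a 2D point stored in FV1X and FV1Y.
; Tick passes through a 0.1-second Delay, re-reads the file, then averages opposite values of the four-number array, apparently a bounding box, and scales the center by a constant.
; A loop over all field names and a print are left disconnected.
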(event `self.ReceiveTick`
  (params (DeltaSeconds :type "Float (single-precision)"))
  (`KismetSystemLibrary.Delay` 0.1)
  (bind _outjsonobject (`JsonBlueprintFunctionLibrary.FromFile` (`self.Json_file`)))
  (bind _fieldnames (`JsonBlueprintFunctionLibrary.GetFieldNames` _outjsonobject))
  (bind _outvalue (`|GetJsonField` _outjsonobject "happy1"))
  (set `self.FV1_X` (* (/ (+ (`|GetArrayItem` _outvalue) (`|GetArrayItem` _outvalue 2)) 2.0) 0.15625))
  (set `self.FV1_Y` (* (/ (+ (`|GetArrayItem` _outvalue 1) (`|GetArrayItem` _outvalue 3)) 2.0) 0.15625)))

(fn `UserConstructionScript`)